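; BP_Tank is a player-controllable tank actor that aims, drives and fires.
; On BeginPlay it passes the barrel and turret to a TankAiming component and both tracks to a TankMovement component.
; Aim axes rotate an azimuth gimbal and spring arm, separating yaw from pitch, while the Fire action calls Fire.
; Forward and turn axes are sent to TankMovement as movement intents.
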(event `self.ReceiveBeginPlay`
  (`TankAimingComponent.Initialize` (`self.TankAiming`) (`self.Barrel`) (`self.TankTurret`))
  (`TankMovementComponent.Initialize` (`self.TankMovement`) (`self.Left_Track`) (`self.Right_Track`)))

(event `InputAxis|AimAzimuth`
  (params (AxisValue :type "Float (single-precision)"))
  ;[1 1 1] Input Mappings
  (`SceneComponent.K2_AddLocalRotation` (`self.AzimuthGimbal`) (`KismetMathLibrary.MakeRotator` 0.0 0.0 AxisValue) false false))

(event `InputAxis|AimElevation`
  (params (AxisValue :type "Float (single-precision)"))
  ;[1 1 1] Input Mappings
  (`SceneComponent.K2_AddLocalRotation` (`self.SpringArm`) (`KismetMathLibrary.MakeRotator` 0.0 (* -1 AxisValue)) false false))

(event `InputAction|Fire`
  (params (Key :type "Key Structure"))
  ;[1 1 1] Input Mappings
  (:`Pressed`
    (`self.Fire`)))

(event `InputAxis|MoveForward`
  (params (AxisValue :type "Float (single-precision)"))
  ;[1 1 1] Input Mappings
  (`TankMovementComponent.IntendMoveFoward` (`self.TankMovement`) AxisValue))

(event `InputAxis|TurnRight`
  (params (AxisValue :type "Float (single-precision)"))
  ;[1 1 1] Input Mappings
  (`TankMovementComponent.IntendTurnRight` (`self.TankMovement`) AxisValue))

(fn `UserConstructionScript`)